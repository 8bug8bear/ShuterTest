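; Climbable ladder-style stairs actor that procedurally builds its mesh along a spline and lets a character attach to it.
; The construction script spawns rungs and side rails at a set step along the spline, plus a collision box scaled to its length.
; Interaction runs a timeline easing the character to the start position, nudged down or up, then enables its on-stairs state if still overlapping.
; Leaving the box clears that state.
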(event OnComponentBeginOverlap(Colision)
  (params (OverlappedComponent :type Primitive%20Component%20Object%20Reference) (OtherActor :type Actor%20Object%20Reference) (OtherComp :type Primitive%20Component%20Object%20Reference) (OtherBodyIndex :type Integer) (bFromSweep :type Boolean) (SweepResult :type Hit%20Result%20Structure%20%28by%20ref%29))
  (bind _asthird_person_character (Utilities|Casting|CastToThirdPersonCharacter OtherActor))
  (Variables|Default|SetCharTemporary _asthird_person_character))

(event OnComponentEndOverlap(Colision)
  (params (OverlappedComponent :type Primitive%20Component%20Object%20Reference) (OtherActor :type Actor%20Object%20Reference) (OtherComp :type Primitive%20Component%20Object%20Reference) (OtherBodyIndex :type Integer))
  (bind _char (Variables|Default|GetChar)
    (:then
      (Default|CharonStairs _char false)
      (Variables|Default|SetCharTemporary 0))
    (:else)))

(event EventIneracterWitnObject
  (params (CharRef :type Third%20Person%20Character%20Object%20Reference))
  (bind _startposition (Variables|Default|GetStartPosition))
  (bind _returnvalue (Transformation|GetWorldLocation _startposition))
  (Variables|Default|SetChar CharRef)
  (bind _output_get (Variables|Default|SetCharDefoultPosition (Transformation|GetWorldLocation (Variables|/Script/Engine.Character|GetCapsuleComponent (Variables|Default|GetChar)))))
  (Variables|Default|SetCharHigherSpline? (> (.z _output_get) (.z (Spline|GetLocationatSplinePoint (Variables|Default|GetSpline) 1 "World"))))
  (bind _newtrack_0 (Timeline|NuveToStairs PlayFromStart)
    (:Update
      (Transformation|SetWorldLocation (Variables|/Script/Engine.Character|GetCapsuleComponent (Variables|Default|GetChar)) (Math|Vector|Lerp(Vector) (Variables|Default|GetCharDefoultPosition) (Math|Vector|MakeVector (.x _returnvalue) (.y _returnvalue) (select (Variables|Default|GetCharHigherSpline?) (- (.Z (Math|Vector|BreakVector (Variables|Default|GetCharDefoultPosition))) 5e+01) (+ (.Z (Math|Vector|BreakVector (Variables|Default|GetCharDefoultPosition))) 5e+01))) _newtrack_0) false false))
    (:Finished
      (if (== (Variables|Default|GetCharTemporary) (Variables|Default|GetChar))
        (Default|CharonStairs (Variables|Default|GetChar) true)))))

(fn ConstructionScript
  (bind _spline (Variables|Default|GetSpline))
  (bind _returnvalue (Spline|GetSplineLength _spline))
  (for _index (range 0 (.ReturnValue (Math|Float|Division(WholeandRemainder) (Spline|GetSplineLength (Variables|Default|GetSpline)) (Variables|Default|GetLengthStep))))
    (Variables|Default|SetFLindex _index)
    ;[1 1 1] Создаём ступеньки
    (AddComponent|AddStaticMeshComponent false (Math|Transform|MakeTransform (Math|Vector|MakeVector 0.0 (Utilities|CalculeteWidthStairs) (Utilities|CalculeteLocationZ (Variables|Default|GetLengthStep))) "0, 0,90.000000" (Math|Vector|MakeVector 0.1 0.1 (/ (Variables|Default|GetWidthStairs) 1e+03))))
    ;[1 1 1] Создаём левый и правый поркчень
    (AddComponent|AddStaticMeshComponent false (Math|Transform|MakeTransform (Math|Vector|MakeVector 0.0 (* (Utilities|CalculeteWidthStairs) -1.0) (- (Utilities|CalculeteLocationZ (Variables|Default|GetLengthStep)) 2e+01)) "0, 0, 0" "0.200000,0.200000,0.500000"))
    (AddComponent|AddStaticMeshComponent false (Math|Transform|MakeTransform (Math|Vector|MakeVector 0.0 (Utilities|CalculeteWidthStairs) (- (Utilities|CalculeteLocationZ (Variables|Default|GetLengthStep)) 2e+01)) "0, 0, 0" "0.200000,0.200000,0.500000")))
  ;[1 1 1] Создание Коллизии
  (bind _returnvalue_2 (AddComponent|AddBoxComponent false (Math|Transform|MakeTransform (Math|Vector|MakeVector -23.0 0.0 (+ (/ (Spline|GetSplineLength (Variables|Default|GetSpline)) 2.0) 1.7e+02)) "0, 0, 0" (Math|Vector|MakeVector 2.0 1.8 (- (/ _returnvalue 5e+01) (/ _returnvalue 2e+02))))))
  (Variables|Default|SetColision _returnvalue_2))